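; BP_Porte is a door that opens or shifts when the player presses F nearby while holding the gold key (Cléeor).
; Entering its Box trigger as BP_Joueur caches the player and enables input on the door, and leaving calls DisableInput through the player controller.
; A valid press plays a 2D door sound and runs a timeline that drives the static mesh's relative location, with no reverse path.
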(event `Key|F`
  (params (Key :type "Key Structure"))
  (:`Pressed`
    (if (`/Game/ThirdPerson/Blueprints/BP_Joueur.Cléeor` (stale `self.Box.OnComponentBeginOverlap` _asbp_joueur))
      (`GameplayStatics.PlaySound2D` "/Game/Jeu/Audio/closing-door-393444.closing-door-393444" 1.0 1.0 0.0 null null)
      (bind (_direction _nouvelle_piste_3) (`Timeline|Chronologie`)
        (:`Update`
          (`SceneComponent.K2_SetRelativeLocation` (`self.StaticMeshComponent`) _nouvelle_piste_3 false false))))))

(event `self.Box.OnComponentBeginOverlap`
  (params (OverlappedComponent :type "PrimitiveComponent Object Reference") (OtherActor :type "Actor Object Reference") (OtherComp :type "PrimitiveComponent Object Reference") (OtherBodyIndex :type Integer) (bFromSweep :type Boolean) (SweepResult :type "HitResult Structure (by ref)"))
  (bind _asbp_joueur (cast `/Game/ThirdPerson/Blueprints/BP_Joueur` OtherActor))
  (`self.EnableInput` (`GameplayStatics.GetPlayerController` 0)))

(event `self.Box.OnComponentEndOverlap`
  (params (OverlappedComponent :type "PrimitiveComponent Object Reference") (OtherActor :type "Actor Object Reference") (OtherComp :type "PrimitiveComponent Object Reference") (OtherBodyIndex :type Integer))
  (cast `/Game/ThirdPerson/Blueprints/BP_Joueur` OtherActor)
  (`self.DisableInput` (`GameplayStatics.GetPlayerController` 0) null))

(fn `UserConstructionScript`)